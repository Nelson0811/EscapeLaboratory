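; BP_BrokenDoor is a two-panel sliding lab door that opens when a BP_Body actor overlaps its Collision component and closes when one leaves.
; Two timelines drive LabDoor03A and LabDoor03B apart in opposite directions along their relative Y axis.
; End overlap reverses both timelines from their current position, with no count of bodies still inside the trigger.
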(event OnComponentBeginOverlap(Collision)
  (params (OverlappedComponent :type Primitive%20Component%20Object%20Reference) (OtherActor :type Actor%20Object%20Reference) (OtherComp :type Primitive%20Component%20Object%20Reference) (OtherBodyIndex :type Integer) (bFromSweep :type Boolean) (SweepResult :type Hit%20Result%20Structure%20%28by%20ref%29))
  ;[0 0.3281 0] SecurityBreach0X00CF52
  (Utilities|Casting|CastToBP_Body OtherActor)
  (Utilities|FlowControl|Sequence
    (:then_0
      (bind _newtrack_0 (Timeline|Timeline Play)
        (:Update
          (Transformation|SetRelativeLocation (Variables|Default|GetLabDoor03B) (Math|Vector|MakeVector 0.0 (* _newtrack_0 9e+01) 0.0) false false))))
    (:then_1
      (bind _newtrack_0_2 (Timeline|Timeline_0 Play)
        (:Update
          (Transformation|SetRelativeLocation (Variables|Default|GetLabDoor03A) (Math|Vector|MakeVector 0.0 (* _newtrack_0_2 -9e+01) 0.0) false false))))))

(event OnComponentEndOverlap(Collision)
  (params (OverlappedComponent :type Primitive%20Component%20Object%20Reference) (OtherActor :type Actor%20Object%20Reference) (OtherComp :type Primitive%20Component%20Object%20Reference) (OtherBodyIndex :type Integer))
  ;[0 0.3281 0] SecurityBreach0X00CF52
  (Utilities|Casting|CastToBP_Body OtherActor)
  (Utilities|FlowControl|Sequence
    (:then_0
      (bind _newtrack_0 (Timeline|Timeline Reverse)
        (:Update
          (Transformation|SetRelativeLocation (Variables|Default|GetLabDoor03B) (Math|Vector|MakeVector 0.0 (* _newtrack_0 9e+01) 0.0) false false))))
    (:then_1
      (bind _newtrack_0_2 (Timeline|Timeline_0 Reverse)
        (:Update
          (Transformation|SetRelativeLocation (Variables|Default|GetLabDoor03A) (Math|Vector|MakeVector 0.0 (* _newtrack_0_2 -9e+01) 0.0) false false))))))

(fn ConstructionScript)