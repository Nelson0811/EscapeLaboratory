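; BP_ExitDoor is a two-panel sliding exit door in the Science Lab that opens for a BP_Body only while its OK flag is set.
; OK starts false and is not set true in this Blueprint; a graph comment ties it to a computer.
; Collision overlap plays the Open and Close timelines together to slide DoorL and DoorR apart along local Y, and end overlap reverses both.
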(event OnComponentBeginOverlap(Collision)
  (params (OverlappedComponent :type Primitive%20Component%20Object%20Reference) (OtherActor :type Actor%20Object%20Reference) (OtherComp :type Primitive%20Component%20Object%20Reference) (OtherBodyIndex :type Integer) (bFromSweep :type Boolean) (SweepResult :type Hit%20Result%20Structure%20%28by%20ref%29))
  ;[1 1 1] Open Door If computer Ok
  (Utilities|Casting|CastToBP_Body OtherActor)
  (if (Variables|Default|GetOK)
    (Utilities|FlowControl|Sequence
      (:then_0
        (bind _newtrack_0 (Timeline|Open Play)
          (:Update
            (Transformation|SetRelativeLocation (Variables|Default|GetDoorL) (Math|Vector|MakeVector 0.0 (* _newtrack_0 9e+01) 0.0) false false))))
      (:then_1
        (bind _newtrack_0_2 (Timeline|Close Play)
          (:Update
            (Transformation|SetRelativeLocation (Variables|Default|GetDoorR) (Math|Vector|MakeVector 0.0 (* _newtrack_0_2 -9e+01) 0.0) false false)))))))

(event OnComponentEndOverlap(Collision)
  (params (OverlappedComponent :type Primitive%20Component%20Object%20Reference) (OtherActor :type Actor%20Object%20Reference) (OtherComp :type Primitive%20Component%20Object%20Reference) (OtherBodyIndex :type Integer))
  ;[1 1 1] Open Door If computer Ok
  (Utilities|Casting|CastToBP_Body OtherActor)
  (if (Variables|Default|GetOK)
    (Utilities|FlowControl|Sequence
      (:then_0
        (bind _newtrack_0 (Timeline|Open Reverse)
          (:Update
            (Transformation|SetRelativeLocation (Variables|Default|GetDoorL) (Math|Vector|MakeVector 0.0 (* _newtrack_0 9e+01) 0.0) false false))))
      (:then_1
        (bind _newtrack_0_2 (Timeline|Close Reverse)
          (:Update
            (Transformation|SetRelativeLocation (Variables|Default|GetDoorR) (Math|Vector|MakeVector 0.0 (* _newtrack_0_2 -9e+01) 0.0) false false)))))))

(event EventBeginPlay
  ;[1 1 1] BeginPlay
  (Variables|Default|SetOK false))

(fn ConstructionScript)