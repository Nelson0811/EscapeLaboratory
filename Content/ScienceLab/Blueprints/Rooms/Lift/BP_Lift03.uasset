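; BP_Lift03 is a one-way science lab lift with two swinging doors that open when a BP_Body enters its collision.
; The first exit from the collision closes the doors and sets a flag that Tick picks up once to start the ascent after a configurable delay.
; One timeline swings the doors, another raises the actor from its starting location, and a delay chained to the movement updates reopens the doors.
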(event OnComponentEndOverlap(Collision)
  (params (OverlappedComponent :type Primitive%20Component%20Object%20Reference) (OtherActor :type Actor%20Object%20Reference) (OtherComp :type Primitive%20Component%20Object%20Reference) (OtherBodyIndex :type Integer))
  (Utilities|Casting|CastToBP_Body OtherActor)
  (Utilities|FlowControl|DoOnce false
    (:Completed
      (Variables|Default|SetOk true)
      (bind _newtrack_0 (Timeline|elevator Reverse)
        (:Update
          (Transformation|SetRelativeRotation (Variables|Default|GetLift02Door02) (Math|Rotator|MakeRotator 0.0 0.0 (* _newtrack_0 9e+01)) false false)
          (Transformation|SetRelativeRotation (Variables|Default|GetLift02Door01) (Math|Rotator|MakeRotator 0.0 0.0 (* _newtrack_0 -9e+01)) false false))))))

(event OnComponentBeginOverlap(Collision)
  (params (OverlappedComponent :type Primitive%20Component%20Object%20Reference) (OtherActor :type Actor%20Object%20Reference) (OtherComp :type Primitive%20Component%20Object%20Reference) (OtherBodyIndex :type Integer) (bFromSweep :type Boolean) (SweepResult :type Hit%20Result%20Structure%20%28by%20ref%29))
  (Utilities|Casting|CastToBP_Body OtherActor)
  (bind _newtrack_0 (Timeline|elevator Play)
    (:Update
      (Transformation|SetRelativeRotation (Variables|Default|GetLift02Door02) (Math|Rotator|MakeRotator 0.0 0.0 (* _newtrack_0 9e+01)) false false)
      (Transformation|SetRelativeRotation (Variables|Default|GetLift02Door01) (Math|Rotator|MakeRotator 0.0 0.0 (* _newtrack_0 -9e+01)) false false))))

(event EventBeginPlay
  ;[1 1 1] beginPlay
  (Variables|Default|SetRelative%20Location (Variables|/Script/Engine.SceneComponent|GetRelativeLocation (Variables|Default|GetDefaultSceneRoot)))
  (Variables|Default|SetOk false))

(event EventTick
  (params (DeltaSeconds :type Float%20%28single-precision%29))
  (bind _relative_location (Variables|Default|GetRelative%20Location))
  ;[1 1 1] tick
  (if (Variables|Default|GetOk)
    (Utilities|FlowControl|DoOnce false
      (:Completed
        (Utilities|FlowControl|Delay (Variables|Default|GetDelayUp))
        (bind _newtrack_0 (Timeline|Timeline Play)
          (:Update
            (Transformation|SetActorLocation (Math|Vector|MakeVector (.x _relative_location) (.y _relative_location) (+ _newtrack_0 (.z _relative_location))) false false)
            (Utilities|FlowControl|Delay 1e+01)
            (bind _newtrack_0_2 (Timeline|elevator Play)
              (:Update
                (Transformation|SetRelativeRotation (Variables|Default|GetLift02Door02) (Math|Rotator|MakeRotator 0.0 0.0 (* _newtrack_0_2 9e+01)) false false)
                (Transformation|SetRelativeRotation (Variables|Default|GetLift02Door01) (Math|Rotator|MakeRotator 0.0 0.0 (* _newtrack_0_2 -9e+01)) false false)))))))))

(fn ConstructionScript)

(fn ElevatorUp)